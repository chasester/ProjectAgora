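; Actor component that tracks health for its owning actor and reports its death.
; Health starts at the maximum on BeginPlay, and the Damage event subtracts from it, clamped at zero.
; On first reaching zero, a DoOnce sends KillMessage to the owner with the victim, damaging actor and impact normal.
; A getter exposes current and maximum health.
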(event `self.ReceiveBeginPlay`
  (set `self.Health` (`self.MaxHealth`)))

(event `/Game/ProjectAgora/Blueprints/Character/BI_HealthStystem.Damage`
  (params (Damage :type "Float (single-precision)") (Actor :type "Actor Object Reference") (Victum :type "Actor Object Reference") (ImpactNormal :type "Vector Structure"))
  (bind _returnvalue (`self.GetOwner` self))
  (bind _output_get (set `self.Health` (`KismetMathLibrary.FMax` 0.0 (- (`self.Health`) Damage))))
  (if (== _output_get 0.0)
    (`/Engine/EditorBlueprintResources/StandardMacros.DoOnce` false
      (:`Completed`
        (message `/Game/ProjectAgora/Blueprints/Character/BI_HealthStystem.Kill` _returnvalue _returnvalue Actor ImpactNormal)))))

(fn `GetCurrentHealth`
  (returns (CurrentHealth :type "Float (double-precision)") (MaxHeath :type "Float (double-precision)"))
  (return (`self.Health`) (`self.MaxHealth`)))