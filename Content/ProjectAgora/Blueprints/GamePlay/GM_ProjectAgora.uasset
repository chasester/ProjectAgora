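; Game mode for a round-based zombie survival game with up to four local players, covering menu reset and restarts.
; Tagged PlayerStarts supply human and zombie spawns, and RoundProfile sets each round's zombie count.
; Kill events remove zombies, score the killer and check for game end, starting the next round once all zombies are gone.
; All players dying or rounds running out shows the end menu with the top scorer.
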(event `self.ReceiveBeginPlay`
  (`self.Gather All Player Starts`)
  (`self.StartNextRound`))

(event `/Game/ProjectAgora/Blueprints/Character/BI_HealthStystem.Kill`
  (params (Victum :type "Actor Object Reference") (Actor :type "Actor Object Reference") (ImpactNormal :type "Vector Structure"))
  (`self.HandleKill` Victum Actor)
  (`self.ShouldGameEnd`))

(event `self.HandleStartingNewPlayer`
  (params (NewPlayer :type "PlayerController Object Reference"))
  (bind _aspc_project_agora (cast `/Game/ProjectAgora/Blueprints/GamePlay/PC_ProjectAgora` NewPlayer :!pure true))
  ;[1 1 1] Get first player - First time
  (bind _returnvalue (`KismetArrayLibrary.Array_AddUnique` (`self.PC_Players`) _aspc_project_agora))
  (if (== _returnvalue 0)
    (`/Game/ProjectAgora/Blueprints/GamePlay/PC_ProjectAgora.AddMainMenu` _aspc_project_agora)))

(event `StartGame`
  (params (NumberOfPlayers :type Integer))
  (for _index (range 1 (`KismetMathLibrary.Clamp` NumberOfPlayers 1 4))
    (bind _returnvalue (`GameplayStatics.CreatePlayer` _index)))
  (set `self.Round` 0)
  (`self.SpawnPlayers`)
  (`KismetSystemLibrary.Delay` 2.0)
  (`self.StartNextRound`))

(event `SpawnZombies`
  (params (LastIndex :type Integer) (Duration :type "Float (double-precision)"))
  (bind _zombiespawns (`self.ZombieSpawns`))
  (for _ (range 1 (+ LastIndex 1))
    (bind _returnvalue (`|SpawnActorFromClass` "/Game/ProjectAgora/Blueprints/Character/P_ZombieCharacter.P_ZombieCharacter_C" (`self.GetTransform` (`|GetArrayItem` _zombiespawns (`KismetMathLibrary.RandomInteger` (`KismetArrayLibrary.Array_Length` _zombiespawns)))) "Undefined" "OverrideRootScale" null null))
    (`KismetArrayLibrary.Array_Add` (`self.CurrentZombies`) (cast `/Game/ProjectAgora/Blueprints/Character/AI/AIC_Zombie` (`Pawn.GetController` _returnvalue) :!pure true))))

(event `Reset`
  ;[1 1 1] If going to main menu
  (`self.RemoveAllExtraPC`)
  (`self.Remove Zombies`)
  (`self.RemoveAllPawns`)
  (set `self.Round` -1)
  (`self.StartNextRound`))

(event `RestartMap`
  (params (Numberofplayers :type Integer))
  (`self.Remove Zombies`)
  (`self.RemoveAllPawns`)
  (`self.StartGame` Numberofplayers))

(fn `CheckPlayerShouldEnd`
  (returns (isAlive :type Boolean))
  (for _array_element (`self.PC_Players`)
    (if (`/Game/ProjectAgora/Blueprints/Character/ThirdPersonCharacter.IsAlive` (cast `/Game/ProjectAgora/Blueprints/Character/ThirdPersonCharacter` (`Controller.K2_GetPawn` _array_element) :!pure true))
      (return false)))
  (return true))

(fn `CheckZombieShouldEnd`
  (returns (`Should End` :type Boolean))
  (if (< (`KismetArrayLibrary.Array_Length` (`self.CurrentZombies`)) 1)
    (bind _nomorerounds (`self.StartNextRound`))
    (if _nomorerounds
      (return true)
      (else
        (return false)))
    (else
      (return false))))

(fn `Gather All Player Starts`
  (`KismetArrayLibrary.Array_Clear` (`self.ZombieSpawns`))
  (`KismetArrayLibrary.Array_Clear` (`self.HumanSpawns`))
  (bind _outactors (`GameplayStatics.GetAllActorsOfClass` "/Script/Engine.PlayerStart"))
  (for _array_element _outactors
    (for _array_element_2 (`Actor.Tags` _array_element)
      (switch `name` _array_element_2
        (:`Zombie`
          (`KismetArrayLibrary.Array_Add` (`self.ZombieSpawns`) _array_element))
        (:`Human`
          (`KismetArrayLibrary.Array_Add` (`self.HumanSpawns`) _array_element))))))

(fn `GetCurrentHealth`
  (returns (CurrentHealth :type "Float (double-precision)") (MaxHeath :type "Float (double-precision)"))
  (return 0.0 0.0))

(fn `GetWinner`
  (returns (ReturnValue :type Integer))
  (locals (Winner :type Integer) (TopScore :type "Float (double-precision)" :default -1.0))
  (for (_array_element _array_index) (`self.PC_Players`)
    (bind _asps_project_agora (cast `/Game/ProjectAgora/Blueprints/GamePlay/PS_ProjectAgora` (`Controller.PlayerState` _array_element) :!pure true))
    (bind _playerscore (`/Game/ProjectAgora/Blueprints/GamePlay/PS_ProjectAgora.PlayerScore` _asps_project_agora))
    (if (> _playerscore (`local.TopScore`))
      (set `local.Winner` _array_index)
      (set `local.TopScore` _playerscore))
    (`/Game/ProjectAgora/Blueprints/GamePlay/PS_ProjectAgora.ResetScore` _asps_project_agora))
  (return (+ (`local.Winner`) 1)))

(fn `HandleKill`
  (params (Victum :type "Actor Object Reference") (Actor :type "Actor Object Reference"))
  (bind _aspawn (cast `Pawn` Victum))
  (bind _aspc_project_agora (cast `/Game/ProjectAgora/Blueprints/GamePlay/PC_ProjectAgora` (`Pawn.GetController` _aspawn))
    (:`then`
      (if (== (`KismetArrayLibrary.Array_Find` (`self.PC_Players`) _aspc_project_agora) -1)
        (`KismetSystemLibrary.PrintString` "ERROR: Player Does Not Exist")))
    (:`CastFailed`
      (bind _asaic_zombie (cast `/Game/ProjectAgora/Blueprints/Character/AI/AIC_Zombie` (`Pawn.GetController` _aspawn)))
      (`KismetArrayLibrary.Array_RemoveItem` (`self.CurrentZombies`) _asaic_zombie)
      (bind _aspawn_2 (cast `Pawn` (`local.Actor`)))
      (bind _asps_project_agora (cast `/Game/ProjectAgora/Blueprints/GamePlay/PS_ProjectAgora` (`Pawn.PlayerState` _aspawn_2)))
      (`/Game/ProjectAgora/Blueprints/GamePlay/PS_ProjectAgora.AddScore` _asps_project_agora 1.0))))

(fn `Remove Zombies`
  (bind _outactors (`GameplayStatics.GetAllActorsOfClass` "/Game/ProjectAgora/Blueprints/Character/P_ZombieCharacter.P_ZombieCharacter_C"))
  (for _array_element _outactors
    (bind _returnvalue (`Pawn.GetController` _array_element))
    (`/Engine/EditorBlueprintResources/StandardMacros.IsValid` _returnvalue
      (:`Is Valid`
        (`Controller.UnPossess` _returnvalue))
      (:`Is Not Valid`
        _))
    (`self.SetLifeSpan` _array_element 0.1))
  (`KismetArrayLibrary.Array_Clear` (`self.CurrentZombies`)))

(fn `RemoveAllExtraPC`
  (bind _pc_players (`self.PC_Players`))
  (bind (_arrayindex _arrayelement) (`/Engine/EditorBlueprintResources/StandardMacros.ReverseForEachLoop` _pc_players)
    (:`LoopBody`
      (if (not (== _arrayindex 0))
        (`self.SetLifeSpan` (`Controller.K2_GetPawn` _arrayelement) 0.1)
        (`Controller.UnPossess` _arrayelement)
        (`GameplayStatics.RemovePlayer` _arrayelement)))
    (:`Completed`
      (`KismetArrayLibrary.Array_Resize` _pc_players 1))))

(fn `RemoveAllPawns`
  (for _array_element (`self.PC_Players`)
    (`self.SetLifeSpan` (`Controller.K2_GetPawn` _array_element) 0.1)
    (`Controller.UnPossess` _array_element)
    (bind _returnvalue (`|SpawnActorFromClass` "/Game/ProjectAgora/Blueprints/Character/P_Emplty.P_Emplty_C" (`KismetMathLibrary.MakeTransform` (0.0 0.0 0.0)) "AdjustIfPossibleButAlwaysSpawn" "OverrideRootScale" null null))
    (`Controller.Possess` _array_element _returnvalue)))

(fn `ShouldGameEnd`
  (bind _output (`|GetArrayItem` (`self.PC_Players`)))
  (if (< (`self.Round`) 1)
    (return)
    (else
      (bind _isalive (`self.CheckPlayerShouldEnd`))
      (if _isalive
        (bind _returnvalue (`self.GetWinner`))
        (`/Game/ProjectAgora/Blueprints/GamePlay/PC_ProjectAgora.AddEndMenu` _output false _returnvalue)
        (set `/Game/ProjectAgora/Blueprints/GamePlay/GS_ProjectAgora.Round` 0 (cast `/Game/ProjectAgora/Blueprints/GamePlay/GS_ProjectAgora` (`GameplayStatics.GetGameState`) :!pure true))
        (else
          (bind _should_end (`self.CheckZombieShouldEnd`))
          (if _should_end
            (bind _returnvalue_2 (`self.GetWinner`))
            (`/Game/ProjectAgora/Blueprints/GamePlay/PC_ProjectAgora.AddEndMenu` _output true _returnvalue_2)))))))

(fn `SpawnPlayers`
  (bind _humanspawns (`self.HumanSpawns`))
  (`KismetArrayLibrary.Array_Shuffle` _humanspawns)
  (for (_array_element _array_index) (`self.PC_Players`)
    (bind _returnvalue (`|SpawnActorFromClass` "/Game/ProjectAgora/Blueprints/Character/P_HumanCharacter.P_HumanCharacter_C" (`self.GetTransform` (`|GetArrayItem` _humanspawns _array_index)) "AdjustIfPossibleButAlwaysSpawn" "OverrideRootScale" null null))
    (`Controller.Possess` _array_element _returnvalue)))

(fn `StartNextRound`
  (returns (NoMoreRounds :type Boolean))
  (bind _round (`self.Round`))
  (bind _roundprofile (`self.RoundProfile`))
  (bind _result (`/Engine/EditorBlueprintResources/StandardMacros.IncrementInt` _round)
    (:`  `
      (if (> _result (`KismetArrayLibrary.Array_LastIndex` _roundprofile))
        (set `/Game/ProjectAgora/Blueprints/GamePlay/GS_ProjectAgora.Round` 0 (cast `/Game/ProjectAgora/Blueprints/GamePlay/GS_ProjectAgora` (`GameplayStatics.GetGameState`) :!pure true))
        (return true)
        (else
          (`self.SpawnZombies` (`|GetArrayItem` _roundprofile _round))
          (set `/Game/ProjectAgora/Blueprints/GamePlay/GS_ProjectAgora.Round` (`self.Round`) (cast `/Game/ProjectAgora/Blueprints/GamePlay/GS_ProjectAgora` (`GameplayStatics.GetGameState`) :!pure true))
          (return false))))))

(fn `UserConstructionScript`)