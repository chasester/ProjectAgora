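; Player controller for Project Agora that manages the game's menus and relays map start and reset requests to GM_ProjectAgora.
; On possess it switches the view to the camera tagged MainCamera and creates the main menu.
; Events show main, end and round-counter widgets, with the main and end menus switching to UI-only input with a visible cursor.
; Kill disables the victim's input, and GetCurrentHealth is a stub returning zeros.
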(event `self.ReceiveBeginPlay`)

(event `self.ReceivePossess`
  (params (PossessedPawn :type "Pawn Object Reference"))
  (bind _outactors (`GameplayStatics.GetAllActorsOfClassWithTag` "/Script/Engine.CameraActor" "MainCamera"))
  (for _array_element _outactors
    (`self.SetViewTargetWithBlend` _array_element)
    (break))
  (bind _returnvalue (`|CreateWidget` "/Game/ProjectAgora/Blueprints/UI/WB_MainMenu.WB_MainMenu_C"))
  (set `self.MainMenu` _returnvalue))

(event `/Game/ProjectAgora/Blueprints/Character/BI_HealthStystem.Kill`
  (params (Victum :type "Actor Object Reference") (Actor :type "Actor Object Reference") (ImpactNormal :type "Vector Structure"))
  (`self.DisableInput` Victum self))

(event `AddMainMenu`
  (bind _mainmenu (`self.MainMenu`))
  (`WidgetLayoutLibrary.RemoveAllWidgets`)
  (`/Engine/EditorBlueprintResources/StandardMacros.IsValid` _mainmenu
    (:`Is Valid`
      _)
    (:`Is Not Valid`
      (bind _returnvalue (`|CreateWidget` "/Game/ProjectAgora/Blueprints/UI/WB_MainMenu.WB_MainMenu_C"))
      (set `self.MainMenu` _returnvalue)))
  (`UserWidget.AddToViewport` _mainmenu 1)
  (`WidgetBlueprintLibrary.SetInputMode_UIOnlyEx` self (`self.MainMenu`))
  (set `self.bShowMouseCursor` true))

(event `AddEndMenu`
  (params (Win :type Boolean) (WinningPlayer :type Integer))
  (bind _endmenu (`self.EndMenu`))
  (`/Engine/EditorBlueprintResources/StandardMacros.IsValid` _endmenu
    (:`Is Valid`
      _)
    (:`Is Not Valid`
      (bind _returnvalue (`|CreateWidget` "/Game/ProjectAgora/Blueprints/UI/WB_EndMenu.WB_EndMenu_C"))
      (bind _output_get (set `self.EndMenu` _returnvalue))))
  (`UserWidget.AddToViewport` _endmenu 1)
  (`/Game/ProjectAgora/Blueprints/UI/WB_EndMenu.SetupVariable` _output_get Win WinningPlayer)
  (`WidgetBlueprintLibrary.SetInputMode_UIOnlyEx` self (`self.MainMenu`))
  (set `self.bShowMouseCursor` true))

(event `RequestStartMap`
  (params (Numberofplayers :type Integer))
  (`/Game/ProjectAgora/Blueprints/GamePlay/GM_ProjectAgora.RestartMap` (cast `/Game/ProjectAgora/Blueprints/GamePlay/GM_ProjectAgora` (`GameplayStatics.GetGameMode`) :!pure true) Numberofplayers))

(event `RequestResetMap`
  (`/Game/ProjectAgora/Blueprints/GamePlay/GM_ProjectAgora.Reset` (cast `/Game/ProjectAgora/Blueprints/GamePlay/GM_ProjectAgora` (`GameplayStatics.GetGameMode`) :!pure true))
  (`self.AddMainMenu`))

(event `AddRoundMenu`
  (params (Round :type Integer))
  (`/Engine/EditorBlueprintResources/StandardMacros.IsValid` null
    (:`Is Valid`
      _)
    (:`Is Not Valid`
      (bind _returnvalue (`|CreateWidget` "/Game/ProjectAgora/Blueprints/UI/WB_HUD_RoundCounter.WB_HUD_RoundCounter_C"))
      (bind _output_get (set `self.RoundMenu` _returnvalue))))
  (`UserWidget.AddToViewport` _output_get 0))

(event `RemoveRoundMenu`
  (`/Engine/EditorBlueprintResources/StandardMacros.IsValid` null
    (:`Is Valid`
      (`Widget.RemoveFromParent` (`self.RoundMenu`)))))

(fn `GetCurrentHealth`
  (returns (CurrentHealth :type "Float (double-precision)") (MaxHeath :type "Float (double-precision)"))
  (return 0.0 0.0))

(fn `UserConstructionScript`)